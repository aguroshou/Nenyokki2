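; Manager actor that keeps a vertically scrolling sprite background continuous by spawning ScrollBackground tiles.
; BeginPlay spawns the first tile, gives it the 1_back sprite and tracks it as the bottom actor.
; Each Tick, once that actor rises to the spawn Z threshold, a new tile spawns one background height below it and becomes the tracked bottom.
; Later tiles keep their class's default sprite.
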(event `self.ReceiveBeginPlay`
  (bind _returnvalue (`|SpawnActorFromClass` "/Game/Aguro/Level/Main/ScrollBackground.ScrollBackground_C" (`KismetMathLibrary.MakeTransform` (0.0 -100.0 0.0)) "Undefined" "OverrideRootScale" null null))
  (`PaperSpriteComponent.SetSprite` (`/Game/Aguro/Level/Main/ScrollBackground.back_Sprite` _returnvalue) "/Game/Aguro/Images/Main/1_back_Sprite.1_back_Sprite")
  (set `self.BackgroundBottomActor` _returnvalue))

(event `self.ReceiveTick`
  (params (DeltaSeconds :type "Float (single-precision)"))
  (bind (_returnvalue_x _returnvalue_y _returnvalue_z) (`KismetMathLibrary.BreakVector` (`self.K2_GetActorLocation` (`self.BackgroundBottomActor`))))
  (if (>= _returnvalue_z (`self.SpawnBackgroundPosZ`))
    (bind _returnvalue (`|SpawnActorFromClass` "/Game/Aguro/Level/Main/ScrollBackground.ScrollBackground_C" (`KismetMathLibrary.MakeTransform` (`KismetMathLibrary.MakeVector` 0.0 -100.0 (- _returnvalue_z (`self.BackgroundHeight`)))) "Undefined" "OverrideRootScale" null null))
    (set `self.BackgroundBottomActor` _returnvalue)))

(fn `UserConstructionScript`)